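; Dandelion seed actor that drifts down at a set fall speed and can be blown around by mouse-driven wind.
; While FallLock is on, Tick eases the physics velocity toward zero horizontally and FallSpeed vertically to fake air resistance.
; MouseWind releases the lock and loops per tick, adding velocity-change impulses along the wind direction until the wind time expires, then restores the lock.
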(event `self.ReceiveBeginPlay`
  (`PrimitiveComponent.SetPhysicsLinearVelocity` (`self.flying_wadding_animation`) (`KismetMathLibrary.MakeVector` 0.0 0.0 (`self.fall_speed`)) false "None"))

(event `self.ReceiveTick`
  (params (DeltaSeconds :type "Float (single-precision)"))
  (bind _delta_seconds (`self.Delta Seconds`))
  (bind (_returnvalue_x _returnvalue_y _returnvalue_z) (`KismetMathLibrary.BreakVector` (`SceneComponent.GetComponentVelocity` (`self.flying_wadding_animation`))))
  (set `self.Delta Seconds` DeltaSeconds)
  (if (`self.fall_lock`)
    (`PrimitiveComponent.SetPhysicsLinearVelocity` (`self.flying_wadding_animation`) (`KismetMathLibrary.MakeVector` (`KismetMathLibrary.FInterpTo_Constant` _returnvalue_x 0.0 _delta_seconds 100.0) (`KismetMathLibrary.FInterpTo_Constant` _returnvalue_y 0.0 _delta_seconds 100.0) (`KismetMathLibrary.FInterpTo_Constant` _returnvalue_z (`self.fall_speed`) _delta_seconds 100.0)) false "None")))

(event `/Game/bp/i_wind.mouse_wind`
  (params (wind_dir :type "Vector Structure") (wind_power :type "Float (double-precision)") (wind_time :type "Float (double-precision)"))
  (bind _returnvalue (- (`self.Wind Time`) (`self.Delta Seconds`)))
  (set `self.fall_lock` false)
  (set `self.Wind Dir` wind_dir)
  (set `self.Wind Power` wind_power)
  (set `self.Wind Time` wind_time)
  (if (> _returnvalue 0.0) :!label _label
    (set `self.Wind Time` _returnvalue)
    (`PrimitiveComponent.AddImpulse` (`self.flying_wadding_animation`) (* (`self.Wind Dir`) (`self.Wind Power`)) "None" true) ; 模拟重力下落
    (`KismetSystemLibrary.DelayUntilNextTick`)
    (goto _label)
    (else
      (set `self.fall_lock` true) ; 吹风结束，恢复蒲公英空气阻力
    )))

(fn `UserConstructionScript`)